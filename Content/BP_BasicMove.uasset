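; Moving platform actor that repeatedly animates its Platform component between its starting location and the location of a Visualiser component.
; On BeginPlay it captures both endpoints and scales the timeline play rate by the inverse of LoopTime.
; Each timeline update lerps the position by Alpha and passes it to an RPC-named move event, which sets the location without sweep.
; When the timeline finishes, it restarts on the next tick.
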(event `self.ReceiveBeginPlay`
  (set `self.TargetLocation` (`SceneComponent.K2_GetComponentLocation` (`self.Visualiser`)))
  (`TimelineComponent.SetPlayRate` (`self.Timeline`) (/ 1.0 (`self.LoopTime`)))
  (set `self.StartingLocation` (`SceneComponent.K2_GetComponentLocation` (`self.Platform`)))
  (bind (_direction _alpha) (`Timeline|Timeline` :!via `PlayFromStart` :!label _label)
    (:`Update`
      (`self.RPC_MoveCube` (`KismetMathLibrary.VLerp` (`self.StartingLocation`) (`self.TargetLocation`) _alpha)))
    (:`Finished`
      (`KismetSystemLibrary.DelayUntilNextTick`)
      (goto _label :!via `PlayFromStart`))))

(event `RPC_MoveCube`
  (params (NewLocation :type "Vector Structure"))
  (`SceneComponent.K2_SetWorldLocation` (`self.Platform`) NewLocation false false))

(fn `UserConstructionScript`)