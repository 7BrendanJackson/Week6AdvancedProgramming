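; BP_BreakawayPlatform is a platform that can be a disguised false floor the player falls through, set by the Breakaway flag.
; The construction script shows breakaway platforms in the false-floor material, then BeginPlay disguises them with the grid material.
; BeginPlay also sets the cube to overlap Pawns if Breakaway, otherwise block them.
; An overlap by BP_ThirdPersonCharacter restores the false-floor material, revealing the trap.
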(event `self.ReceiveBeginPlay`
  (bind _cube (`self.Cube`))
  ;[1 1 1] Set collision if the platform breaks
  (`PrimitiveComponent.SetCollisionResponseToChannel` _cube "ECC_Pawn" (select `bool` (`self.Breakaway?`) :`false` "ECR_Block" :`true` "ECR_Overlap" :!type "ECollisionResponse Enum"))
  (`PrimitiveComponent.SetMaterial` _cube 0 "/Engine/OpenWorldTemplate/LandscapeMaterial/MI_ProcGrid.MI_ProcGrid"))

(event `self.Cube.OnComponentBeginOverlap`
  (params (OverlappedComponent :type "PrimitiveComponent Object Reference") (OtherActor :type "Actor Object Reference") (OtherComp :type "PrimitiveComponent Object Reference") (OtherBodyIndex :type Integer) (bFromSweep :type Boolean) (SweepResult :type "HitResult Structure (by ref)"))
  ;[1 1 1] Change material if a player falls through
  (cast `/Game/Blueprints/BP_ThirdPersonCharacter` OtherActor)
  (`PrimitiveComponent.SetMaterial` (`self.Cube`) 0 "/Game/Materials/M_FalseFloor.M_FalseFloor"))

(fn `UserConstructionScript`
  (`PrimitiveComponent.SetMaterial` (`self.Cube`) 0 (select `bool` (`self.Breakaway?`) :`false` "/Engine/OpenWorldTemplate/LandscapeMaterial/MI_ProcGrid.MI_ProcGrid" :`true` "/Game/Materials/M_FalseFloor.M_FalseFloor" :!type "MaterialInterface Object Reference")))