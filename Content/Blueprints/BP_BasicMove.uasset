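; Moving platform Blueprint that repeatedly animates its Platform component between its starting location and the location of a Visualiser component.
; On BeginPlay, only the authority caches both locations, scales the Timeline play rate by LoopTime and calls the MoveCube RPC.
; That event's Timeline lerps the platform without sweeping and restarts one tick after finishing.
; The RPC's NewLocation parameter is unused.
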(event `self.ReceiveBeginPlay`
  (`/Engine/EditorBlueprintResources/ActorMacros.Switch Has Authority`
    (:`Authority`
      (set `self.TargetLocation` (`SceneComponent.K2_GetComponentLocation` (`self.Visualiser`)))
      (`TimelineComponent.SetPlayRate` (`self.Timeline`) (/ 1.0 (`self.LoopTime`)))
      (set `self.StartingLocation` (`SceneComponent.K2_GetComponentLocation` (`self.Platform`)))
      (`self.RPC_MoveCube` (0.0 0.0 0.0)))))

(event `RPC_MoveCube`
  (params (NewLocation :type "Vector Structure"))
  (bind (_direction _alpha) (`Timeline|Timeline` :!via `PlayFromStart` :!label _label)
    (:`Update`
      (`SceneComponent.K2_SetWorldLocation` (`self.Platform`) (`KismetMathLibrary.VLerp` (`self.StartingLocation`) (`self.TargetLocation`) _alpha) false false))
    (:`Finished`
      (`KismetSystemLibrary.DelayUntilNextTick`)
      (goto _label :!via `PlayFromStart`))))

(fn `UserConstructionScript`)